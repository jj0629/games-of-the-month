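; BikeWall is a wall actor, apparently left by a bike, that stretches from a stored start point toward a moving end point.
; UpdateWall sets the BoxCollider extent from the X offset between the points, then scales WallMesh to that extent relative to its original width.
; It zeroes the actor's rotation during resizing and restores it afterward.
; The event graph and construction script are empty, so updates depend on external calls.
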(event EventBeginPlay)

(event Collision|EventActorBeginOverlap
  (params (OtherActor :type Actor%20Object%20Reference)))

(event EventTick
  (params (DeltaSeconds :type Float%20%28single-precision%29)))

(fn ConstructionScript)

(fn UpdateWall
  (params (New%20End%20Point :type Vector))
  (bind _box_collider (Variables|Default|GetBox%20Collider))
  ;[1 0.1818 0.98] Grab original rotation, then reset rotation
  (Variables|Default|SetStart%20Rotation (Transformation|GetActorRotation))
  (Transformation|SetActorRotation "0, 0, 0")
  ;[1 0.7455 0.1227] Set box collider extents
  (bind _output_get (Variables|Default|SetEnd%20Point New%20End%20Point))
  (Components|Box|SetBoxExtent _box_collider (Math|Vector|MakeVector (.X (Class|KismetMathLibrary|BreakVector3f (- _output_get (Variables|Default|GetStart%20Point)))) 25.0 5e+01) true)
  ;[0 0.9907 1] Set wall mesh's scale
  (Transformation|SetRelativeScale3D (Variables|Default|GetWall%20Mesh) (Math|Vector|MakeVector (.X (Class|KismetMathLibrary|BreakVector3f (/ (Variables|/Script/Engine.BoxComponent|GetBoxExtent _box_collider) (Variables|Default|GetOriginal%20Mesh%20Width)))) 0.5 1.0))
  ;[0 0.1057 1] Reset wall's rotation
  (Transformation|SetActorRotation (Variables|Default|GetStart%20Rotation)))