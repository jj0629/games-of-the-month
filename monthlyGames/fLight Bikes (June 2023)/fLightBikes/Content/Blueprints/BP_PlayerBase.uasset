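; BP_PlayerBase is a player-controlled bike that constantly moves forward, driven by Enhanced Input.
; BeginPlay adds the BikeControls mapping context to the player controller.
; Tick pushes movement along ShapeCube's forward vector, while Turn adds right and forward input relative to the same cube and prints its value for debugging.
; CameraLook feeds controller yaw and pitch; a camera zoom move is present but disconnected.
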(event EventBeginPlay)

(event Collision|EventActorBeginOverlap
  (params (OtherActor :type Actor%20Object%20Reference)))

(event EventTick
  (params (DeltaSeconds :type Float%20%28single-precision%29)))

(event Input|EnhancedActionEvents|EnhancedInputActionCameraZoom
  (params (ActionValue :type Float%20%28double-precision%29) (ElapsedSeconds :type Float%20%28double-precision%29) (TriggeredSeconds :type Float%20%28double-precision%29) (InputAction :type Input%20Action%20Object%20Reference :default "/Game/Inputs/CameraZoom.CameraZoom"))
  ;[1 0.8986 0.1146] Zoom Logic
)

(event Input|EnhancedActionEvents|EnhancedInputActionCameraLook
  (params (ActionValue :type Vector%202D%20Structure) (ElapsedSeconds :type Float%20%28double-precision%29) (TriggeredSeconds :type Float%20%28double-precision%29) (InputAction :type Input%20Action%20Object%20Reference :default "/Game/Inputs/CameraLook.CameraLook"))
  (bind (_x _y) (Math|Vector2D|BreakVector2D ActionValue))
  ;[0.157 0.1143 0.6198] Look Logic
  (:Triggered
    (Pawn|Input|AddControllerYawInput _x)
    (Pawn|Input|AddControllerPitchInput _y)))

(event Input|EnhancedActionEvents|EnhancedInputActionTurn
  (params (ActionValue :type Vector%202D%20Structure) (ElapsedSeconds :type Float%20%28double-precision%29) (TriggeredSeconds :type Float%20%28double-precision%29) (InputAction :type Input%20Action%20Object%20Reference :default "/Game/Inputs/Turn.Turn"))
  (bind (_x _y) (Math|Vector2D|BreakVector2D ActionValue))
  (bind _shape_cube (Variables|Default|GetShape_Cube))
  (bind _returnvalue (Transformation|GetWorldRotation _shape_cube))
  (:Triggered
    (Development|PrintText (Utilities|Text|ToText(String) ActionValue))
    (Pawn|Input|AddMovementInput (Math|Vector|GetRightVector _returnvalue) _x false)
    (Pawn|Input|AddMovementInput (Math|Vector|GetForwardVector _returnvalue) _y false)))

(event EventTick
  (params (DeltaSeconds :type Float%20%28single-precision%29))
  ;[1 0.1146 0.2444] Move Bike Forward (Always Active)
  (Pawn|Input|AddMovementInput (Math|Vector|GetForwardVector (Transformation|GetWorldRotation (Variables|Default|GetShape_Cube))) 1.0 false))

(event EventBeginPlay
  ;[1 0.09375 0.7945] Set Input Mappiing Context (Bind Input Map)
  (bind _asplayer_controller (Utilities|Casting|CastToPlayerController (Pawn|GetController)))
  (Input|AddMappingContext (PlayerController|LocalPlayerSubsystems|GetEnhancedInputLocalPlayerSubsystem _asplayer_controller) "/Game/Inputs/BikeControls.BikeControls" 0 "(bIgnoreAllPressedKeysUntilRelease=True,bForceImmediately=False)"))

(fn ConstructionScript)