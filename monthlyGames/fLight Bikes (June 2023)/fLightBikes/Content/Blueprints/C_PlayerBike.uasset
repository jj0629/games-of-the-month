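; Player bike input Blueprint that handles steering and the follow camera for the first player's pawn.
; BeginPlay caches that pawn and its spring arm, which Enhanced Input events then drive.
; Turn applies swept local yaw and pitch to the pawn, while zoom changes arm length.
; Look orbits the arm around world Z and its own right vector, and reset zeroes its world rotation rather than aligning it to the bike.
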(event Input|EnhancedActionEvents|EnhancedInputActionCameraZoom
  (params (ActionValue :type Float%20%28double-precision%29) (ElapsedSeconds :type Float%20%28double-precision%29) (TriggeredSeconds :type Float%20%28double-precision%29) (InputAction :type Input%20Action%20Object%20Reference :default "/Game/Inputs/CameraZoom.CameraZoom"))
  (bind _pawn_spring_arm (Variables|Default|GetPawn%20Spring%20Arm))
  ;[0 1 0.9016] Camera Zoom
  (:Triggered
    (Variables|/Script/Engine.SpringArmComponent|SetTargetArmLength _pawn_spring_arm (+ (* ActionValue (Variables|Default|GetCamera%20Zoom%20Rate)) (Variables|/Script/Engine.SpringArmComponent|GetTargetArmLength _pawn_spring_arm)))))

(event Input|EnhancedActionEvents|EnhancedInputActionCameraLook
  (params (ActionValue :type Vector%202D%20Structure) (ElapsedSeconds :type Float%20%28double-precision%29) (TriggeredSeconds :type Float%20%28double-precision%29) (InputAction :type Input%20Action%20Object%20Reference :default "/Game/Inputs/CameraLook.CameraLook"))
  (bind (_x _y) (Math|Vector2D|BreakVector2D ActionValue))
  (bind _pawn_spring_arm (Variables|Default|GetPawn%20Spring%20Arm))
  ;[0 0.06418 1] Camera Look
  (:Triggered
    (Transformation|AddWorldRotation _pawn_spring_arm (Math|Vector|RotatorfromAxisandAngle "0.000000,0.000000,1.000000" _x) false false)
    (Transformation|AddWorldRotation _pawn_spring_arm (Math|Vector|RotatorfromAxisandAngle (Math|Vector|GetRightVector _pawn_spring_arm) _y) false false)))

(event Input|EnhancedActionEvents|EnhancedInputActionTurn
  (params (ActionValue :type Vector%202D%20Structure) (ElapsedSeconds :type Float%20%28double-precision%29) (TriggeredSeconds :type Float%20%28double-precision%29) (InputAction :type Input%20Action%20Object%20Reference :default "/Game/Inputs/Turn.Turn"))
  (bind (_x _y) (Math|Vector2D|BreakVector2D ActionValue))
  ;[1 0 0.2573] Bike Turn
  (:Triggered
    (Transformation|AddActorLocalRotation (Variables|Default|GetPlayer%20Pawn) (Math|Rotator|MakeRotator 0.0 (* _y (Variables|Default|GetTurn%20Rate)) (* (Variables|Default|GetTurn%20Rate) _x)) true false)))

(event Input|EnhancedActionEvents|EnhancedInputActionCameraReset
  (params (ActionValue :type Boolean) (ElapsedSeconds :type Float%20%28double-precision%29) (TriggeredSeconds :type Float%20%28double-precision%29) (InputAction :type Input%20Action%20Object%20Reference :default "/Game/Inputs/CameraReset.CameraReset"))
  ;[0.9453 1 0.04501] Camera Reset
  (:Triggered
    (Transformation|SetWorldRotation (Variables|Default|GetPawn%20Spring%20Arm) "0, 0, 0" false false)))

(event EventBeginPlay
  (bind _returnvalue (Game|Player|GetPlayerPawn 0))
  (Variables|Default|SetPlayer%20Pawn _returnvalue)
  (Variables|Default|SetPawn%20Spring%20Arm (Actor|GetComponentbyClass _returnvalue "/Script/Engine.SpringArmComponent")))

(fn ConstructionScript)